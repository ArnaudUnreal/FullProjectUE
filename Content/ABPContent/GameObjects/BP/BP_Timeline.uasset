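; BP_Timeline is a demo actor that uses Timelines to animate its mesh color and its rotation.
; On BeginPlay it adds a W_Timeline widget owned by PC_Timeline to the viewport and stores the starting rotation.
; Three events play Timelines: one drives material Color and Alpha parameters, one adds a track to StartRotation, and one lerps toward NewRotation.
; Both rotation events combine rotators on finish, with author notes flagging only the lerp version as working.
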(event `self.ReceiveBeginPlay`
  ;[0 1 0.2261] BeginPlay
  (bind _aspc_timeline (cast `/Game/ABPContent/GameObjects/Game/PC_Timeline` (`GameplayStatics.GetPlayerController` 0)))
  (bind _returnvalue (`|CreateWidget` "/Game/ABPContent/UMG/W_Timeline.W_Timeline_C" _aspc_timeline))
  (`UserWidget.AddToViewport` _returnvalue 0)
  (`UserWidget.SetDesiredSizeInViewport` _returnvalue (320.0 250.0))
  (set `self.StartRotation` (`self.K2_GetActorRotation`)))

(event `eventChangeColor`
  (bind _staticmesh (`self.StaticMesh`))
  ;[1 1 1] Change Color
  (bind (_direction _colortrack) (`Timeline|tl_Color` :!via `PlayFromStart`)
    (:`Update`
      (bind _output_get (set `self.Color Track` _colortrack))
      (`MeshComponent.SetVectorParameterValueOnMaterials` _staticmesh "Color" (`KismetMathLibrary.MakeVector` (break `LinearColor` _output_get) (`.G` (break `LinearColor` _output_get)) (`.B` (break `LinearColor` _output_get))))
      (`MeshComponent.SetScalarParameterValueOnMaterials` _staticmesh "Alpha" (`.A` (break `LinearColor` _output_get))))))

(event `eventRotate`
  (bind _newrotation (`self.NewRotation`))
  ;[1 1 1] Rotate
  (bind (_direction _rotation _lerptrack) (`Timeline|tl_Rotation` :!via `PlayFromStart`)
    (:`Update`
      (bind _output_get (set `self.Rotation` _rotation))
      (set `self.Lerp Track` _lerptrack)
      (bind (_returnvalue_x _returnvalue_y _returnvalue_z) (`KismetMathLibrary.BreakVector` (+ _output_get (`self.StartRotation`))))
      (`self.K2_SetActorRotation` (`KismetMathLibrary.MakeRotator` _returnvalue_x _returnvalue_y _returnvalue_z)))
    (:`Finished`
      ;;[1 0 0.02407] Not Working. Why ?
      (bind _output_get_2 (set `self.StartRotation` (`KismetMathLibrary.ComposeRotators` (`self.StartRotation`) _newrotation)))
      (set `self.NewRotation` (`KismetMathLibrary.ComposeRotators` _output_get_2 _newrotation)))))

(event `eventChangeRotation`
  (bind _newrotation (`self.NewRotation`))
  ;[1 1 1] Change Rotation
  (bind (_direction _lerptrack) (`Timeline|tl_ChangeRotation` :!via `PlayFromStart`)
    (:`Update`
      (`self.K2_SetActorRotation` (`KismetMathLibrary.RLerp` (`self.StartRotation`) (`self.NewRotation`) _lerptrack)))
    (:`Finished`
      ;;[0 1 0.1946] Working. Why ?
      (bind _output_get (set `self.StartRotation` (`KismetMathLibrary.ComposeRotators` (`self.StartRotation`) _newrotation)))
      (set `self.NewRotation` (`KismetMathLibrary.ComposeRotators` _output_get _newrotation)))))

(fn `UserConstructionScript`)