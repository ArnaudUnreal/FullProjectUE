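; BP_WhiteClown is an actor that demonstrates Blueprint interface interaction through I_Interact, showing info via its ACInfos component on BeginPlay only in LineTraceLevel.
; A detection event draws a horizontal Visibility line trace at a set height along the player controller's yaw and sends InteractMessage to a hit actor implementing the interface.
; A separate event broadcasts InteractMessage to every actor in the level that implements I_Interact.
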(event `self.ReceiveBeginPlay`
  ;[0 1 0.2838] BeginPlay
  (bind _returnvalue (`GameplayStatics.GetCurrentLevelName` true))
  (if (== _returnvalue "LineTraceLevel")
    (`/Game/ABPContent/GameObjects/Components/AC_Infos.eventDisplayInfos` (`self.AC_Infos`))))

(event `eventDetectInteraction`
  (bind _returnvalue (`self.K2_GetActorLocation`))
  (bind _traceheight (`self.TraceHeight`))
  (bind (_x _y) (`KismetMathLibrary.BreakVector3f` _returnvalue))
  (bind (_x_2 _y_2) (`KismetMathLibrary.BreakVector3f` _returnvalue))
  (bind (_returnvalue_x _returnvalue_y) (`KismetMathLibrary.BreakVector` (`KismetMathLibrary.GetForwardVector` (`Controller.GetControlRotation` (`GameplayStatics.GetPlayerController` 0)))))
  ;[1 1 1] Detects if the front actor implements an Interface
  (set `self.TraceStartLocation` (`KismetMathLibrary.MakeVector` _x _y _traceheight))
  (set `self.TraceEndLocation` (+ (`KismetMathLibrary.MakeVector` _x_2 _y_2 _traceheight) (* (`KismetMathLibrary.MakeVector` _returnvalue_x _returnvalue_y) (`self.TraceDistance`))))
  (bind (_outhit _returnvalue_2) (`KismetSystemLibrary.LineTraceSingle` :`Start` (`self.TraceStartLocation`) :`End` (`self.TraceEndLocation`) :`TraceChannel` "TraceTypeQuery1" :`DrawDebugType` "ForDuration"))
  (if _returnvalue_2
    (bind (_bblockinghit _binitialoverlap _time _distance _location _impactpoint _normal _impactnormal _physmat _hitactor) (`GameplayStatics.BreakHitResult` _outhit))
    (if (`KismetSystemLibrary.DoesImplementInterface` _hitactor "/Game/ABPContent/GameObjects/Interfaces/I_Interact.I_Interact_C")
      (message `/Game/ABPContent/GameObjects/Interfaces/I_Interact.Interact` _hitactor))))

(event `eventActivateAll`
  ;[1 1 1] Triggers all actors with Interface
  (bind _outactors (`GameplayStatics.GetAllActorsWithInterface` "/Game/ABPContent/GameObjects/Interfaces/I_Interact.I_Interact_C"))
  (for _array_element _outactors
    (message `/Game/ABPContent/GameObjects/Interfaces/I_Interact.Interact` _array_element)))

(fn `UserConstructionScript`)