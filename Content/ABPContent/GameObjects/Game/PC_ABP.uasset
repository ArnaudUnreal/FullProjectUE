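; Player controller that turns Enhanced Input actions into camera and character controls for BP_WhiteClown.
; On BeginPlay it adds movement, mouse and interaction mapping contexts, caches the clown and sets walk speed.
; Handles camera-relative movement, jump, hold-to-run and toggle crouch, broadcasting walking state through a dispatcher.
; Forwards interaction and line-trace detection to the clown and its detection component; holding Switch temporarily swaps mesh and AnimBP to Claire.
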(event `self.ReceiveBeginPlay`
  (bind _returnvalue (subsystem `EnhancedInputLocalPlayerSubsystem`))
  ;[0 1 0.01118 1 20] START
  (`/Engine/EditorBlueprintResources/StandardMacros.IsValid` _returnvalue
    (:`Is Valid`
      (`EnhancedInputSubsystemInterface.AddMappingContext` _returnvalue "/Game/ABPContent/Inputs/IMC_Moves.IMC_Moves" 0 (struct))
      (`EnhancedInputSubsystemInterface.AddMappingContext` _returnvalue "/Game/ABPContent/Inputs/IMC_Mouse.IMC_Mouse" 0 (struct))
      (`EnhancedInputSubsystemInterface.AddMappingContext` _returnvalue "/Game/ABPContent/Inputs/IMC_Interaction.IMC_Interaction" 0 (struct))
      (bind _asbp_white_clown (cast `/Game/ABPContent/GameObjects/BP/BP_WhiteClown` (`GameplayStatics.GetPlayerCharacter` 0)))
      (bind _output_get (set `self.As BP White Clown` _asbp_white_clown))
      (set `CharacterMovementComponent.MaxWalkSpeed` 200.0 (`Character.CharacterMovement` _output_get)))))

(event `EnhancedInput|/Game/ABPContent/Inputs/Actions/IA_Run`
  (params (ActionValue :type Boolean) (ElapsedSeconds :type "Float (double-precision)") (TriggeredSeconds :type "Float (double-precision)") (InputAction :type "InputAction Object Reference" :default "/Game/ABPContent/Inputs/Actions/IA_Run.IA_Run"))
  (bind _charactermovement (`Character.CharacterMovement` (`GameplayStatics.GetPlayerCharacter` 0)))
  ;[1 1 1] INPUTS
  ;;[1 1 1] CHARACTER
  (:`Started`
    (set `CharacterMovementComponent.MaxWalkSpeed` 600.0 _charactermovement))
  (:`Completed`
    (set `CharacterMovementComponent.MaxWalkSpeed` 200.0 _charactermovement)))

(event `EnhancedInput|/Game/ABPContent/Inputs/Actions/IA_InteractAll`
  (params (ActionValue :type Boolean) (ElapsedSeconds :type "Float (double-precision)") (TriggeredSeconds :type "Float (double-precision)") (InputAction :type "InputAction Object Reference" :default "/Game/ABPContent/Inputs/Actions/IA_InteractAll.IA_InteractAll"))
  ;[1 1 1] INPUTS
  ;;[1 1 1] CHARACTER
  (:`Triggered`
    (`/Game/ABPContent/GameObjects/BP/BP_WhiteClown.eventActivateAll` (`self.As BP White Clown`))))

(event `EnhancedInput|/Game/ABPContent/Inputs/Actions/IA_Orbit`
  (params (ActionValue :type "Vector2D Structure") (ElapsedSeconds :type "Float (double-precision)") (TriggeredSeconds :type "Float (double-precision)") (InputAction :type "InputAction Object Reference" :default "/Game/ABPContent/Inputs/Actions/IA_Orbit.IA_Orbit"))
  ;[1 1 1] INPUTS
  ;;[1 1 1] CAMERA
  (:`Triggered`
    (`self.AddYawInput` ActionValue_X)
    (`self.AddPitchInput` ActionValue_Y)))

(event `EnhancedInput|/Game/ABPContent/Inputs/Actions/IA_Jump`
  (params (ActionValue :type Boolean) (ElapsedSeconds :type "Float (double-precision)") (TriggeredSeconds :type "Float (double-precision)") (InputAction :type "InputAction Object Reference" :default "/Game/ABPContent/Inputs/Actions/IA_Jump.IA_Jump"))
  (bind _returnvalue (`GameplayStatics.GetPlayerCharacter` 0))
  ;[1 1 1] INPUTS
  ;;[1 1 1] CHARACTER
  (:`Started`
    (`Character.Jump` _returnvalue))
  (:`Completed`
    (`Character.StopJumping` _returnvalue)))

(event `EnhancedInput|/Game/ABPContent/Inputs/Actions/IA_Interact`
  (params (ActionValue :type Boolean) (ElapsedSeconds :type "Float (double-precision)") (TriggeredSeconds :type "Float (double-precision)") (InputAction :type "InputAction Object Reference" :default "/Game/ABPContent/Inputs/Actions/IA_Interact.IA_Interact"))
  ;[1 1 1] INPUTS
  ;;[1 1 1] CHARACTER
  (:`Triggered`
    (`/Game/ABPContent/GameObjects/BP/BP_WhiteClown.eventDetectInteraction` (`self.As BP White Clown`))))

(event `EnhancedInput|/Game/ABPContent/Inputs/Actions/IA_Crouch`
  (params (ActionValue :type Boolean) (ElapsedSeconds :type "Float (double-precision)") (TriggeredSeconds :type "Float (double-precision)") (InputAction :type "InputAction Object Reference" :default "/Game/ABPContent/Inputs/Actions/IA_Crouch.IA_Crouch"))
  (bind _returnvalue (`GameplayStatics.GetPlayerCharacter` 0))
  ;[1 1 1] INPUTS
  ;;[1 1 1] CHARACTER
  (:`Started`
    (`/Engine/EditorBlueprintResources/StandardMacros.FlipFlop`
      (:`A`
        (`Character.Crouch` _returnvalue))
      (:`B`
        (`Character.UnCrouch` _returnvalue)))))

(event `EnhancedInput|/Game/ABPContent/Inputs/Actions/IA_Moves`
  (params (ActionValue :type "Vector2D Structure") (ElapsedSeconds :type "Float (double-precision)") (TriggeredSeconds :type "Float (double-precision)") (InputAction :type "InputAction Object Reference" :default "/Game/ABPContent/Inputs/Actions/IA_Moves.IA_Moves"))
  (bind _returnvalue (`GameplayStatics.GetPlayerCharacter` 0))
  (bind (_returnvalue_roll _returnvalue_pitch _returnvalue_yaw) (`KismetMathLibrary.BreakRotator` (`self.GetControlRotation`)))
  ;[1 1 1] INPUTS
  ;;[1 1 1] CHARACTER
  (:`Triggered`
    (`Pawn.AddMovementInput` _returnvalue (`KismetMathLibrary.GetRightVector` (`KismetMathLibrary.MakeRotator` _returnvalue_roll 0.0 _returnvalue_yaw)) ActionValue_X false)
    (`Pawn.AddMovementInput` _returnvalue (`KismetMathLibrary.GetForwardVector` (`KismetMathLibrary.MakeRotator` 0.0 0.0 _returnvalue_yaw)) ActionValue_Y false)
    (set `self.IsWalking` true)
    (`self.ED_IsWalking` (`self.IsWalking`) :!label _label))
  (:`Completed`
    (set `self.IsWalking` false)
    (goto _label)))

(event `EnhancedInput|/Game/ABPContent/Inputs/Actions/IA_LineTrace`
  (params (ActionValue :type Boolean) (ElapsedSeconds :type "Float (double-precision)") (TriggeredSeconds :type "Float (double-precision)") (InputAction :type "InputAction Object Reference" :default "/Game/ABPContent/Inputs/Actions/IA_LineTrace.IA_LineTrace"))
  (bind _ac_detection (`/Game/ABPContent/GameObjects/BP/BP_WhiteClown.AC_Detection` (`self.As BP White Clown`)))
  ;[1 1 1] INPUTS
  ;;[1 1 1] CHARACTER
  (:`Triggered`
    (`/Game/ABPContent/GameObjects/Components/AC_Detection.eventDetect` _ac_detection))
  (:`Completed`
    (`/Game/ABPContent/GameObjects/Components/AC_Detection.eventStopDetect` _ac_detection)))

(event `EnhancedInput|/Game/ABPContent/Inputs/Actions/IA_Switch`
  (params (ActionValue :type Boolean) (ElapsedSeconds :type "Float (double-precision)") (TriggeredSeconds :type "Float (double-precision)") (InputAction :type "InputAction Object Reference" :default "/Game/ABPContent/Inputs/Actions/IA_Switch.IA_Switch"))
  (bind _mesh (`Character.Mesh` (`GameplayStatics.GetPlayerCharacter` 0)))
  (:`Started`
    (`|ExecutionSequence`
      (:`then_0`
        (`SkeletalMeshComponent.SetSkeletalMeshAsset` _mesh "/Game/ABPContent/Meshes/SKM/Claire/claire.claire"))
      (:`then_1`
        (`SkeletalMeshComponent.SetAnimInstanceClass` _mesh "/Game/ABPContent/Meshes/SKM/Claire/ABP_claire_Skeleton_AnimBlueprint.ABP_claire_Skeleton_AnimBlueprint_C"))))
  (:`Completed`
    (`|ExecutionSequence`
      (:`then_0`
        (`SkeletalMeshComponent.SetSkeletalMeshAsset` _mesh "/Game/ABPContent/Meshes/SKM/WhiteClown/Whiteclown_N_Hallin.Whiteclown_N_Hallin"))
      (:`then_1`
        (`SkeletalMeshComponent.SetAnimInstanceClass` _mesh "/Game/ABPContent/Meshes/SKM/WhiteClown/ABP_Whiteclown.ABP_Whiteclown_C")))))

(fn `UserConstructionScript`)