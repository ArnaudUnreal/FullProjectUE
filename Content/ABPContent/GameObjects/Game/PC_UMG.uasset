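; Player controller for UMG-based play that lets the player trigger pause through the HUD.
; On BeginPlay, if the Enhanced Input subsystem is valid, it adds the pause mapping context, sets Game and UI input with a visible cursor, and caches the UMG_HUD.
; The pause action calls EventPause on that HUD; its FlipFlop has no branch-specific logic, so any toggling is not done here.
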(event `self.ReceiveBeginPlay`
  (bind _returnvalue (subsystem `EnhancedInputLocalPlayerSubsystem`))
  (`parent.ReceiveBeginPlay`)
  (`/Engine/EditorBlueprintResources/StandardMacros.IsValid` _returnvalue
    (:`Is Valid`
      (`EnhancedInputSubsystemInterface.AddMappingContext` _returnvalue "/Game/ABPContent/Inputs/IMC_Pause.IMC_Pause" 0 (struct))
      (`WidgetBlueprintLibrary.SetInputMode_GameAndUIEx` self null "DoNotLock" false)
      (set `self.bShowMouseCursor` true)
      (bind _asumg_hud (cast `/Game/ABPContent/GameObjects/Game/UMG_HUD` (`self.GetHUD`)))
      (set `self.As UMG HUD` _asumg_hud))))

(event `EnhancedInput|/Game/ABPContent/Inputs/Actions/IA_Pause`
  (params (ActionValue :type Boolean) (ElapsedSeconds :type "Float (double-precision)") (TriggeredSeconds :type "Float (double-precision)") (InputAction :type "InputAction Object Reference" :default "/Game/ABPContent/Inputs/Actions/IA_Pause.IA_Pause"))
  (:`Started`
    (`/Engine/EditorBlueprintResources/StandardMacros.FlipFlop`
      (:`A`
        _)
      (:`B`
        _))
    (`/Game/ABPContent/GameObjects/Game/UMG_HUD.eventPause` (`self.As UMG HUD`))))

(fn `UserConstructionScript`
  (`parent.UserConstructionScript`))