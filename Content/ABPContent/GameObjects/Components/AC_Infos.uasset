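; Actor component that shows its owner's collision responses to trace channels in a W_ObstacleChannels widget.
; When eventDisplayInfos fires, it caches the owner's child skeletal mesh, static mesh and widget components.
; It maps trace types to collision channels by matching enum names, then sends each response to the widget, preferring the skeletal mesh.
; On BeginPlay it also disables on-screen messages via console command.
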(event `self.ReceiveBeginPlay`
  (`KismetSystemLibrary.ExecuteConsoleCommand` "disableallscreenmessages" null))

(event `eventDisplayInfos`
  (for _array_element (`SceneComponent.GetChildrenComponents` (`Actor.RootComponent` (`self.GetOwner`)) true)
    (bind _asskeletal_mesh_component (cast `SkeletalMeshComponent` _array_element)
      (:`then`
        (set `self.SKMCompo` _asskeletal_mesh_component))
      (:`CastFailed`
        (bind _asstatic_mesh_component (cast `StaticMeshComponent` _array_element)
          (:`then`
            (set `self.SMCompo` _asstatic_mesh_component))
          (:`CastFailed`
            (bind _aswidget_component (cast `WidgetComponent` _array_element))
            (set `self.Widget` _aswidget_component))))))
  (bind _enumvalue (foreach `ECollisionChannel` false)
    (:`LoopBody`
      (`KismetArrayLibrary.Array_Add` (`self.CollisionsChannelsArray`) (`|GetEnumeratorNameAsString` _enumvalue))
      (`KismetArrayLibrary.Array_Add` (`self.CollisionsChannelsArrayEnums`) _enumvalue))
    (:`then`
      (bind _enumvalue_2 (foreach `ETraceTypeQuery` true)
        (:`LoopBody`
          (bind _returnvalue (`|GetEnumeratorNameAsString` _enumvalue_2))
          (`KismetArrayLibrary.Array_Add` (`self.TraceTypesArray`) _returnvalue)
          (`KismetArrayLibrary.Array_Add` (`self.TraceTypesArrayEnums`) _enumvalue_2)
          (bind _returnvalue_2 (`KismetArrayLibrary.Array_Find` (`self.CollisionsChannelsArray`) _returnvalue))
          (if (!= _returnvalue_2 -1)
            (bind _skmcompo (`self.SKMCompo`)
              (:`then`
                (bind _output (`|GetArrayItem` (`self.CollisionsChannelsArrayEnums`) _returnvalue_2))
                (`self.SetDatas` _returnvalue _skmcompo _output))
              (:`else`
                (bind _smcompo (`self.SMCompo`)
                  (:`then`
                    (`self.SetDatas` _returnvalue _smcompo _output))
                  (:`else`))))))))))

(fn `SetDatas`
  (params (Datas_Channel :type String) (Component :type "PrimitiveComponent Object Reference") (Channel :type "ECollisionChannel Enum" :default "ECC_WorldStatic"))
  (bind _output_get (set `self.Channel Datas` (make `/Game/ABPContent/Datas/Structs/S_ResponseChannel` Datas_Channel (`|GetEnumeratorNameAsString` (`PrimitiveComponent.GetCollisionResponseToChannel` Component Channel)))))
  (bind _asw_obstacle_channels (cast `/Game/ABPContent/UMG/W_ObstacleChannels` (`WidgetComponent.GetWidget` (`self.Widget`))))
  (`/Game/ABPContent/UMG/W_ObstacleChannels.AddDatas` _asw_obstacle_channels _output_get)
  (return))