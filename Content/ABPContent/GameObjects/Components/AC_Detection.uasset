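; Detection component that line-traces at a fixed height to find BP_Projectile actors and activate their projectile movement, apparently as a trace-channel demo.
; eventDetect runs a debug-drawn single or multi trace from the owner, ending at the player's flattened control direction scaled from world origin, not the owner.
; BP_WhiteClown owners also get a 3D label naming the trace channel.
; eventStopDetect flushes debug lines, and BeginPlay disables on-screen messages.
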(event `self.ReceiveBeginPlay`
  (`KismetSystemLibrary.ExecuteConsoleCommand` "disableallscreenmessages" null))

(event `eventDetect`
  (bind _returnvalue (`Actor.K2_GetActorLocation` (`self.GetOwner`)))
  (bind (_returnvalue_x _returnvalue_y) (`KismetMathLibrary.BreakVector` (`KismetMathLibrary.GetForwardVector` (`Controller.GetControlRotation` (`GameplayStatics.GetPlayerController` 0)))))
  (bind (_x _y) (`KismetMathLibrary.BreakVector3f` _returnvalue))
  (bind (_x_2 _y_2) (`KismetMathLibrary.BreakVector3f` _returnvalue))
  (bind (_returnvalue_x_2 _returnvalue_y_2) (`KismetMathLibrary.BreakVector` (* (`KismetMathLibrary.MakeVector` _returnvalue_x _returnvalue_y) 10000.0)))
  (bind _asbp_white_clown (cast `/Game/ABPContent/GameObjects/BP/BP_WhiteClown` (`self.GetOwner`))
    (:`then`
      (bind _returnvalue_2 (`|AddComponentByClass` _asbp_white_clown "/Script/Engine.TextRenderComponent" false (`KismetMathLibrary.MakeTransform` (0.0 100.0 0.0) (struct :`Yaw` 180.0) (0.2 0.2 0.2))))
      (bind _output_get (set `self.Text3D` _returnvalue_2))
      (`TextRenderComponent.K2_SetText` _output_get (`KismetTextLibrary.Conv_StringToText` (`KismetStringLibrary.Concat_StrStr` "Current Trace Channel : " (`|GetEnumeratorNameAsString` (`self.Trace Channel`)))))
      (`TextRenderComponent.SetTextRenderColor` _returnvalue_2 (make `Color` 0 0 1 1)))
    (:`CastFailed`
      _))
  (set `self.TraceStartLocation` (`KismetMathLibrary.MakeVector` _x _y 20.0))
  (set `self.TraceEndLocation` (+ (`KismetMathLibrary.MakeVector` _x_2 _y_2 20.0) (* (`KismetMathLibrary.MakeVector` _returnvalue_x _returnvalue_y) 200.0)))
  (set `self.MultiTraceEndLocation` (`KismetMathLibrary.MakeVector` _returnvalue_x_2 _returnvalue_y_2 20.0))
  (if (`self.Multi?`)
    (bind _outhits (`KismetSystemLibrary.LineTraceMulti` :`Start` (`self.TraceStartLocation`) :`End` (`self.MultiTraceEndLocation`) :`TraceChannel` (`self.Trace Channel`) :`DrawDebugType` "ForDuration" :`TraceColor` (struct :`R` 0.002615 :`B` 1.0 :`A` 1.0) :`TraceHitColor` (struct :`R` 1.0 :`G` 0.043423 :`B` 0.655114 :`A` 1.0)))
    (if (> (`KismetArrayLibrary.Array_Length` _outhits) 0)
      (for _array_element _outhits
        (bind _asbp_projectile (cast `/Game/ABPContent/GameObjects/BP/BP_Projectile` (`.HitActor` (`GameplayStatics.BreakHitResult` _array_element))))
        (`KismetSystemLibrary.Delay` 0.5)
        (`self.Activate` (`/Game/ABPContent/GameObjects/BP/BP_Projectile.ProjectileMovement` _asbp_projectile) false)))
    (else
      (bind (_outhit _returnvalue_3) (`KismetSystemLibrary.LineTraceSingle` :`Start` (`self.TraceStartLocation`) :`End` (`self.MultiTraceEndLocation`) :`TraceChannel` (`self.Trace Channel`) :`DrawDebugType` "ForDuration"))
      (if _returnvalue_3
        (bind (_bblockinghit _binitialoverlap _time _distance _location _impactpoint _normal _impactnormal _physmat _hitactor) (`GameplayStatics.BreakHitResult` _outhit))
        (`KismetSystemLibrary.PrintString` (`KismetSystemLibrary.GetDisplayName` _hitactor))
        (bind _asbp_projectile_2 (cast `/Game/ABPContent/GameObjects/BP/BP_Projectile` _hitactor))
        (if (`KismetSystemLibrary.DoesImplementInterface` _hitactor)
          (`self.Activate` (`/Game/ABPContent/GameObjects/BP/BP_Projectile.ProjectileMovement` _asbp_projectile_2) false))))))

(event `eventStopDetect`
  (`KismetSystemLibrary.FlushPersistentDebugLines`))